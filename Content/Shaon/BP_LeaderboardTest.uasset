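; BP_LeaderboardTest is a trigger actor for testing the leaderboard.
; When BP_FirstPersonCharacter_Shaon overlaps its Box, it submits that character's points and name to BPACLeaderboard with a hardcoded placeholder time.
; It then passes the component's scores and names back to the character for display.
; Disconnected nodes remain, including a cast to BP_FirstPersonCharacter_Master.
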(event `self.Box.OnComponentBeginOverlap`
  (params (OverlappedComponent :type "PrimitiveComponent Object Reference") (OtherActor :type "Actor Object Reference") (OtherComp :type "PrimitiveComponent Object Reference") (OtherBodyIndex :type Integer) (bFromSweep :type Boolean) (SweepResult :type "HitResult Structure (by ref)"))
  (bind _bpac_leaderboard (`self.BPAC_Leaderboard`))
  (bind _asbp_first_person_character_shaon (cast `/Game/Shaon/BP_FirstPersonCharacter_Shaon` OtherActor))
  (`/Game/Shaon/BPAC_Leaderboard.Update Leaderboard` (`self.BPAC_Leaderboard`) (`/Game/Shaon/BP_FirstPersonCharacter_Shaon.Points` _asbp_first_person_character_shaon) (`/Game/Shaon/BP_FirstPersonCharacter_Shaon.PlayerName` _asbp_first_person_character_shaon) "00:00.001")
  (`/Game/Shaon/BP_FirstPersonCharacter_Shaon.Display leaderboard` :`self` _asbp_first_person_character_shaon :`Scoreboard` (`/Game/Shaon/BPAC_Leaderboard.Leaderboard Scores` _bpac_leaderboard) :`Names` (`/Game/Shaon/BPAC_Leaderboard.Leaderboard Names` _bpac_leaderboard)))

(fn `UserConstructionScript`)