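; BP_SouthParkBull is an AI bull character that wanders randomly and charges a player carrying a cube.
; It repeats random reachable moves with random pauses, bobbing its mesh on a sine wave while grounded to fake hopping.
; Detection-sphere overlap raises walk speed and starts the chase, while stun-wall contact halts movement.
; Perception updates only store a target; focus logic is disconnected and nothing follows the stun delay.
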(event `self.ReceiveBeginPlay`
  ; Bull AI wander
  (`self.MoveToRandomLocation`))

(event `MoveToRandomLocation`
  ; Bull AI wander
  (`|AIMoveTo` self (`NavigationSystemV1.K2_GetRandomReachablePointInRadius` (`self.K2_GetActorLocation`) 1000.0 null null) null
    (:`then`
      (`KismetSystemLibrary.Delay` (`KismetMathLibrary.RandomFloatInRange` 0.5 2.5))
      (`self.MoveToRandomLocation`))))

(event `self.ReceiveTick`
  (params (DeltaSeconds :type "Float (single-precision)"))
  ; Hopping Code AI
  (if (`NavMovementComponent.IsMovingOnGround` (`self.CharacterMovement`))
    (`SceneComponent.K2_SetRelativeLocation` (`self.Mesh`) (`KismetMathLibrary.MakeVector` 0.0 0.0 (* (`KismetMathLibrary.Sin` (* (`KismetSystemLibrary.GetGameTimeInSeconds`) 25.0)) 20.0)) false false)))

(event `self.DetectionSphere.OnComponentBeginOverlap`
  (params (OverlappedComponent :type "PrimitiveComponent Object Reference") (OtherActor :type "Actor Object Reference") (OtherComp :type "PrimitiveComponent Object Reference") (OtherBodyIndex :type Integer) (bFromSweep :type Boolean) (SweepResult :type "HitResult Structure (by ref)"))
  ; AI Charge Player
  (bind _asbp_first_person_character (cast `/Game/Characters/FirstPerson/Blueprints/BP_FirstPersonCharacter` OtherActor))
  (if (`/Game/Characters/FirstPerson/Blueprints/BP_FirstPersonCharacter.bHasCube` _asbp_first_person_character)
    (bind _output_get (set `self.As BP First Person Character` _asbp_first_person_character))
    (set `CharacterMovementComponent.MaxWalkSpeed` 1000.0 (`self.CharacterMovement`))
    (`|AIMoveTo` self (0.0 0.0 0.0) _output_get)))

(event `self.NPCAI.OnTargetPerceptionUpdated`
  (params (Actor :type "Actor Object Reference") (Stimulus :type "AIStimulus Structure"))
  ; Targeting Perception
  (set `self.TargetActor` Actor))

(event `self.Mesh.OnComponentBeginOverlap`
  (params (OverlappedComponent :type "PrimitiveComponent Object Reference") (OtherActor :type "Actor Object Reference") (OtherComp :type "PrimitiveComponent Object Reference") (OtherBodyIndex :type Integer) (bFromSweep :type Boolean) (SweepResult :type "HitResult Structure (by ref)"))
  ; Stun
  (cast `/Game/JP_Dev/Migration/scene/StaticMeshes/BP_StunWall` OtherActor)
  (`MovementComponent.StopMovementImmediately` (`self.CharacterMovement`))
  (`KismetSystemLibrary.Delay` 2.0))

(fn `UserConstructionScript`)