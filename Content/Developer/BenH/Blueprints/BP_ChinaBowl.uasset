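; BP_ChinaBowl is a physics-simulated china bowl the first-person character can pick up.
; Trigger overlaps cache the character and set its ChinaGrab flag, though leaving also sets it true.
; Grab stops physics, attaches the sphere to the character's hold spot, updates its carry state and count, and calls ChinaSpeed.
; Shatter logic (Niagara effect, breaking sound, destroy) is present but disconnected.
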(event `Grab`
  (bind _sphere (`self.Sphere`))
  ; Grab Custom Event code. Honestly might be bad :(
  (if (`/Game/Developer/BenH/Characters/BP_FirstPersonCharacter_Master_BenCopy.HasChina?` (stale `self.PickupTrigger.OnComponentBeginOverlap` _asbp_first_person_character_master_ben_copy))
    _
    (elif (`/Game/Developer/BenH/Characters/BP_FirstPersonCharacter_Master_BenCopy.ChinaGrab` (stale `self.PickupTrigger.OnComponentBeginOverlap` _asbp_first_person_character_master_ben_copy))
      (`PrimitiveComponent.SetSimulatePhysics` (`self.Sphere`) false)
      (bind _chinaholdspot (`/Game/Developer/BenH/Characters/BP_FirstPersonCharacter_Master_BenCopy.ChinaHoldSpot` (stale `self.PickupTrigger.OnComponentBeginOverlap` _asbp_first_person_character_master_ben_copy)))
      (`SceneComponent.K2_SetWorldLocation` _sphere (`SceneComponent.K2_GetComponentLocation` _chinaholdspot) false false)
      (`SceneComponent.K2_AttachToComponent` _sphere _chinaholdspot "None" "KeepWorld" "KeepWorld" "KeepWorld" true)
      (set `/Game/Developer/BenH/Characters/BP_FirstPersonCharacter_Master_BenCopy.ChinaItemCount` (+ (`/Game/Developer/BenH/Characters/BP_FirstPersonCharacter_Master_BenCopy.ChinaItemCount` (stale `self.PickupTrigger.OnComponentBeginOverlap` _asbp_first_person_character_master_ben_copy)) 1) (stale `self.PickupTrigger.OnComponentBeginOverlap` _asbp_first_person_character_master_ben_copy))
      (set `/Game/Developer/BenH/Characters/BP_FirstPersonCharacter_Master_BenCopy.HasChina?` true (stale `self.PickupTrigger.OnComponentBeginOverlap` _asbp_first_person_character_master_ben_copy))
      (`/Game/Developer/BenH/Characters/BP_FirstPersonCharacter_Master_BenCopy.ChinaSpeed` (stale `self.PickupTrigger.OnComponentBeginOverlap` _asbp_first_person_character_master_ben_copy)))))

(event `self.ReceiveBeginPlay`
  (`PrimitiveComponent.SetSimulatePhysics` (`self.Sphere`) true))

(event `self.PickupTrigger.OnComponentBeginOverlap`
  (params (OverlappedComponent :type "PrimitiveComponent Object Reference") (OtherActor :type "Actor Object Reference") (OtherComp :type "PrimitiveComponent Object Reference") (OtherBodyIndex :type Integer) (bFromSweep :type Boolean) (SweepResult :type "HitResult Structure (by ref)"))
  (bind _asbp_first_person_character_master_ben_copy (cast `/Game/Developer/BenH/Characters/BP_FirstPersonCharacter_Master_BenCopy` OtherActor))
  (set `/Game/Developer/BenH/Characters/BP_FirstPersonCharacter_Master_BenCopy.ChinaGrab` true _asbp_first_person_character_master_ben_copy)
  (`KismetSystemLibrary.PrintString` "You Can pick me up"))

(event `self.PickupTrigger.OnComponentEndOverlap`
  (params (OverlappedComponent :type "PrimitiveComponent Object Reference") (OtherActor :type "Actor Object Reference") (OtherComp :type "PrimitiveComponent Object Reference") (OtherBodyIndex :type Integer))
  (bind _asbp_first_person_character_master_ben_copy (cast `/Game/Developer/BenH/Characters/BP_FirstPersonCharacter_Master_BenCopy` OtherActor))
  (set `/Game/Developer/BenH/Characters/BP_FirstPersonCharacter_Master_BenCopy.ChinaGrab` true _asbp_first_person_character_master_ben_copy)
  (`KismetSystemLibrary.PrintString` "You can no longer pick me up"))

(fn `UserConstructionScript`)